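; Enemy spawner actor that keeps creating BP_Enemy instances at its own transform while its live count is below MaxCnt.
; A looping timer, with its interval randomized once at BeginPlay, calls SpawnEnemy, which increments NowCnt and prints it for debugging.
; Each enemy's BPEnemyFSM receives a reference to the spawner, which exposes MinusNowCnt to decrement the count without going below zero.
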(event `self.ReceiveBeginPlay`
  (`KismetSystemLibrary.K2_SetTimer` null "SpawnEnemy" (`KismetMathLibrary.RandomFloatInRange` 1.0 2.0) true)
  (`KismetSystemLibrary.PrintString` "spawn stop" true false))

(fn `AddNowCnt`
  (set `self.NowCnt` (+ (`self.NowCnt`) 1)))

(fn `MinusNowCnt`
  (if (!= (`self.NowCnt`) 0)
    (set `self.NowCnt` (- (`self.NowCnt`) 1))))

(fn `SpawnEnemy`
  (if (< (`self.NowCnt`) (`self.MaxCnt`))
    (bind _returnvalue (`|SpawnActorFromClass` "/Game/Blueprint/BP_Enemy.BP_Enemy_C" (`self.GetTransform`) "Undefined" "MultiplyWithRoot" null null))
    (`|ExecutionSequence`
      (:`then_0`
        (`self.AddNowCnt`)
        (`KismetSystemLibrary.PrintString` (`KismetStringLibrary.Conv_IntToString` (`self.NowCnt`)) true false))
      (:`then_1`
        (set `/Game/Blueprint/BP_EnemyFSM.SpawnerRef` self (`/Game/Blueprint/BP_Enemy.BP_EnemyFSM` _returnvalue))))))

(fn `UserConstructionScript`)